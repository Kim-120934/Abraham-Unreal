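; Interactive door that either swings or slides, toggled open and closed by Interact through SetOpen.
; A timeline sized to AnimDuration plays forward or in reverse, and BeginPlay sets its time to match the initial IsOpen state.
; The timeline update scales normalized playback position by OpenRange to drive DoorPivot's yaw or local Y offset, chosen by IsRotator, without needing a curve track.
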(event EventBeginPlay
  (bind _openclosetimeline (Variables|Default|GetOpenCloseTimeline))
  (Components|Timeline|SetTimelineLength (Variables|Default|GetOpenCloseTimeline) (Variables|Default|GetAnimDuration))
  (if (Variables|Default|GetIsOpen)
    (Components|Timeline|SetNewTime _openclosetimeline (Components|Timeline|GetTimelineLength _openclosetimeline))
    (else
      (Components|Timeline|SetNewTime _openclosetimeline 0.0))))

(event EventInteract
  (bind _output_get (Variables|Default|SetIsOpen (not (Variables|Default|GetIsOpen))))
  (CallFunction|SetOpen _output_get))

(fn ConstructionScript)

(fn SetOpen
  (params (SetOpen :type Boolean))
  (bind _openclosetimeline (Variables|Default|GetOpenCloseTimeline))
  (if SetOpen
    (Audio|Components|Audio|Play _openclosetimeline)
    (else
      (Utilities|String|Reverse _openclosetimeline))))